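; Saving strategy that persists and restores the state of an InteractiveSceneObject through a BP_InteractiveObjectSaveGame.
; Save copies the actor's location, scale, type and BP_ColorComponent color into the save object.
; Load writes them back, teleporting the actor without sweep; rotation is not stored.
; Both functions cast owner and save object first, returning true only after copying completes.
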(fn `Load`
  (params (Owner :type "Actor Object Reference (by ref)") (SaveGame :type "SaveGame Object Reference"))
  (returns (Success :type Boolean))
  (locals (Object :type "InteractiveSceneObject Object Reference"))
  (bind _asinteractive_scene_object (cast `InteractiveSceneObject` Owner))
  (set `local.Object` _asinteractive_scene_object)
  (bind _asbp_interactive_object_save_game (cast `/Game/InteractiveObject/SaveGame/BP_InteractiveObjectSaveGame` SaveGame))
  (`Actor.K2_SetActorLocation` (`local.Object`) (`/Game/InteractiveObject/SaveGame/BP_InteractiveObjectSaveGame.Location` _asbp_interactive_object_save_game) false true)
  (`Actor.SetActorScale3D` (`local.Object`) (`/Game/InteractiveObject/SaveGame/BP_InteractiveObjectSaveGame.Scale` _asbp_interactive_object_save_game))
  (`/Game/GeneralComponents/BP_ColorComponent.SetColor` (`Actor.GetComponentByClass` (`local.Object`) "/Game/GeneralComponents/BP_ColorComponent.BP_ColorComponent_C") (`/Game/InteractiveObject/SaveGame/BP_InteractiveObjectSaveGame.Color` _asbp_interactive_object_save_game))
  (set `InteractiveSceneObject.Type` (`/Game/InteractiveObject/SaveGame/BP_InteractiveObjectSaveGame.Type` _asbp_interactive_object_save_game) (`local.Object`))
  (return true))

(fn `Save`
  (params (Owner :type "Actor Object Reference (by ref)") (SaveGameObj :type "SaveGame Object Reference"))
  (returns (Success :type Boolean))
  (locals (Objects :type "InteractiveSceneObject Object Reference"))
  (bind _asinteractive_scene_object (cast `InteractiveSceneObject` Owner))
  (set `local.Objects` _asinteractive_scene_object)
  (bind _asbp_interactive_object_save_game (cast `/Game/InteractiveObject/SaveGame/BP_InteractiveObjectSaveGame` SaveGameObj))
  (set `/Game/InteractiveObject/SaveGame/BP_InteractiveObjectSaveGame.Location` (`Actor.K2_GetActorLocation` (`local.Objects`)) _asbp_interactive_object_save_game)
  (set `/Game/InteractiveObject/SaveGame/BP_InteractiveObjectSaveGame.Scale` (`Actor.GetActorScale3D` (`local.Objects`)) _asbp_interactive_object_save_game)
  (set `/Game/InteractiveObject/SaveGame/BP_InteractiveObjectSaveGame.Color` (`/Game/GeneralComponents/BP_ColorComponent.GetColor` (`Actor.GetComponentByClass` (`local.Objects`) "/Game/GeneralComponents/BP_ColorComponent.BP_ColorComponent_C")) _asbp_interactive_object_save_game)
  (set `/Game/InteractiveObject/SaveGame/BP_InteractiveObjectSaveGame.Type` (`InteractiveSceneObject.Type` (`local.Objects`)) _asbp_interactive_object_save_game)
  (return true))