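; BP_InteractiveObject is an interactive object whose static mesh changes color at runtime.
; On BeginPlay it blocking-loads its material, creates a dynamic instance stored as ObjectMaterial and applies it to the mesh's first slot.
; When BP_ColorComponent fires OnColorChanged, it sets the "Color" vector parameter on the mesh's dynamic materials.
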(event `self.ReceiveBeginPlay`
  (bind _returnvalue (`KismetSystemLibrary.LoadAsset_Blocking` (`self.Material`)))
  (bind _asmaterial_interface (cast `MaterialInterface` _returnvalue))
  (bind _returnvalue_2 (`KismetMaterialLibrary.CreateDynamicMaterialInstance` _asmaterial_interface))
  (bind _output_get (set `self.ObjectMaterial` _returnvalue_2))
  (`PrimitiveComponent.SetMaterial` (`self.StaticMeshComponent`) 0 _output_get))

(event `self.BP_ColorComponent.OnColorChanged`
  (params (NewColor :type "LinearColor Structure (by ref)"))
  (for _array_element (`MeshComponent.GetMaterials` (`self.StaticMeshComponent`))
    (bind _asmaterial_instance_dynamic (cast `MaterialInstanceDynamic` _array_element))
    (`MaterialInstanceDynamic.SetVectorParameterValue` _asmaterial_instance_dynamic "Color" NewColor)))

(fn `UserConstructionScript`)