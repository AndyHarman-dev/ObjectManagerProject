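; BP_SavingComponent is an actor component that saves and loads its owner's state through a pluggable strategy object.
; On BeginPlay it async-loads and constructs the strategy class, and loads the configured slot's SaveGame or async-loads its class to create one.
; Save has the strategy fill that object, then writes it to the slot if successful.
; Load hands the cached object to the strategy without rereading the slot.
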(event `self.ReceiveBeginPlay`
  (`self.AsyncSetStratgy`)
  (`self.AsyncSetSaveGameObject`))

(event `AsyncSetStratgy`
  (bind _class (`|LoadAssetClass` (`self.StrategyClass`))
    (:`Completed`
      (bind _asbp_saving_strategy_base (castclass `/Game/GeneralComponents/SavingComponent/BP_SavingStrategyBase` _class)
        (:`then`
          (bind _returnvalue (`|GenericCreateObject` _asbp_saving_strategy_base))
          (set `self.Strategy` _returnvalue))
        (:`CastFailed`
          (`KismetSystemLibrary.LogString` "error: couldn't load strategy class!"))))))

(event `AsyncSetSaveGameObject`
  (bind _savegameinfo_class (break `/Game/GeneralComponents/SavingComponent/S_SaveGameInfo` (`self.SaveGameInfo`)))
  (bind (_savegameinfo_class_2 _savegameinfo_slotname) (break `/Game/GeneralComponents/SavingComponent/S_SaveGameInfo` (`self.SaveGameInfo`)))
  (bind (_savegameinfo_class_3 _savegameinfo_slotname_2) (break `/Game/GeneralComponents/SavingComponent/S_SaveGameInfo` (`self.SaveGameInfo`)))
  (bind _returnvalue (`GameplayStatics.DoesSaveGameExist` _savegameinfo_slotname_2))
  (if _returnvalue
    (bind _returnvalue_2 (`GameplayStatics.LoadGameFromSlot` _savegameinfo_slotname))
    (set `self.SaveGameObject` _returnvalue_2)
    (else
      (bind _class (`|LoadAssetClass` _savegameinfo_class)
        (:`Completed`
          (bind _assave_game (castclass `SaveGame` _class))
          (bind _returnvalue_3 (`GameplayStatics.CreateSaveGameObject` _assave_game))
          (set `self.SaveGameObject` _returnvalue_3))))))

(fn `Load`
  (returns (Success :type Boolean))
  (bind _strategy (`self.Strategy`)
    (:`then`
      (bind _success (`/Game/GeneralComponents/SavingComponent/BP_SavingStrategyBase.Load` _strategy (`self.GetOwner`) (`self.SaveGameObject`)))
      (return _success))
    (:`else`
      (`KismetSystemLibrary.LogString` "error: saving strategy is invalid!"))))

(fn `Save`
  (returns (Success :type Boolean))
  (bind (_savegameinfo_class _savegameinfo_slotname) (break `/Game/GeneralComponents/SavingComponent/S_SaveGameInfo` (`self.SaveGameInfo`)))
  (bind _strategy (`self.Strategy`)
    (:`then`
      (bind _success (`/Game/GeneralComponents/SavingComponent/BP_SavingStrategyBase.Save` _strategy (`self.GetOwner`) (`self.SaveGameObject`)))
      (if _success
        (bind _returnvalue (`GameplayStatics.SaveGameToSlot` (`self.SaveGameObject`) _savegameinfo_slotname))
        (return _returnvalue)
        (else
          (return false))))
    (:`else`
      (`KismetSystemLibrary.LogString` "error: saving strategy is invalid!"))))